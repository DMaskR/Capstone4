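; Timer is a countup game clock that ends the match with a Game Over screen once it passes 1:59.
; Tick runs through a one-second Delay, using the latent node as a throttle to increment Seconds and roll it over into Minutes.
; At the limit it adds the Game_Over widget to the viewport, shows the mouse cursor and pauses the game.
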(event EventBeginPlay)

(event EventTick
  (params (DeltaSeconds :type Float%20%28single-precision%29))
  (Utilities|FlowControl|Delay 1.0)
  (if (== (Variables|Default|Getseconds) 59)
    (if (== (Variables|Default|Getminutes) 1)
      (bind _returnvalue (UserInterface|CreateWidget "/Game/Blueprints/Game_Over.Game_Over_C"))
      (UserInterface|Viewport|AddtoViewport _returnvalue 0)
      (Variables|/Script/Engine.PlayerController|SetbShowMouseCursor (Game|GetPlayerController 0) true)
      (Game|SetGamePaused true)
      (else
        (Variables|Default|Setseconds 0)
        (Variables|Default|Setminutes (+ (Variables|Default|Getminutes) 1))))
    (else
      (Variables|Default|Setseconds (+ (Variables|Default|Getseconds) 1)))))

(fn ConstructionScript)