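; Enemy AI pawn that wanders between random reachable points and shoots at the player on sight.
; Tick drives AI MoveTo while alive and not firing, picking a new nearby point after a random pause.
; PawnSensing turns it toward the player and, after a random delay, spawns an aimed bullet if ammo remains.
; AI Perception toggles firing, and losing sight redirects movement to a random point near the player's current location.
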(event OnSeePawn(PawnSensing)
  (params (Pawn :type Pawn%20Object%20Reference))
  ;[1 1 1] When we see the player, turn to him and fire bullet
  (if (not (not (Variables|Default|GetIsAlive?)))
    (Variables|Default|SetCanFire? true)
    (Transformation|SetActorRotation (Math|Rotator|FindLookatRotation (Transformation|GetActorLocation) (Transformation|GetActorLocation (Game|GetPlayerCharacter 0))))
    (Utilities|FlowControl|Delay (Math|Random|RandomFloatinRange 0.2 1.5))
    (CallFunction|FireBullet)))

(event OnTargetPerceptionUpdated(AIPerception)
  (params (Actor :type Actor%20Object%20Reference) (Stimulus :type AI%20Stimulus%20Structure))
  ;[1 1 1] If player lost sight / go to last seen players loc
  (if (.bSuccessfullySensed (Utilities|Struct|BreakAIStimulus Stimulus))
    (Variables|Default|SetCanFire? true)
    (else
      (Variables|Default|SetCanFire? false)
      (CallFunction|GotoLastPlayerLoc))))

(event Custom|FindAPointToGo
  (Variables|Default|SetLocationToGo (.RandomLocation (AI|Navigation|GetRandomReachablePointinRadius (Transformation|GetActorLocation) 1e+03 0 0))))

(event Custom|GoToLastPlayerLoc
  ;[1 1 1] Find a random position where the player was before losing his track
  (Variables|Default|SetLocationToGo (.RandomLocation (AI|Navigation|GetRandomReachablePointinRadius (Transformation|GetActorLocation (Game|GetPlayerCharacter 0)) 5e+02 0 0))))

(event Custom|FireBullet
  (bind _bulletspawn (Variables|Default|GetBulletSpawn))
  (bind _returnvalue (Transformation|GetWorldLocation _bulletspawn))
  ;[1 1 1] Spawn bullet to the player
  (bind _haveenoughmunitions_ (CallFunction|CheckMunitionsLeft))
  (if _haveenoughmunitions_
    (Collision|LineTraceByChannel (Transformation|GetWorldLocation (Variables|Default|GetBulletSpawn)) (Transformation|GetActorLocation (Game|GetPlayerCharacter 0)) "TraceTypeQuery1" false 0 "ForDuration")
    (Game|SpawnActorfromClass "/Game/Blueprints/BP_Bullets.BP_Bullets_C" (Math|Transform|MakeTransform _returnvalue (Math|Rotator|FindLookatRotation _returnvalue (Transformation|GetActorLocation (Game|GetPlayerCharacter 0))) "5.000000,5.000000,5.000000") "Undefined" 0 0)
    (CallFunction|DecreasingMunitions)))

(event EventBeginPlay
  (|CallParentFunction)
  (Variables|Default|SetLocationToGo (.RandomLocation (AI|Navigation|GetRandomReachablePointinRadius (Transformation|GetActorLocation) 1e+03 0 0))))

(event EventTick
  (params (DeltaSeconds :type Float%20%28single-precision%29))
  ;[1 1 1] Aimove to
  (if (not (not (Variables|Default|GetIsAlive?)))
    (if (not (Variables|Default|GetCanFire?))
      (AI|AIMoveTo (Pawn|GetControlledPawn (Pawn|GetController)) (Variables|Default|GetLocationToGo) 0 5.0 false
        (:OnSuccess
          (Utilities|FlowControl|Delay (Math|Random|RandomFloatinRange 1.0 3.0))
          (CallFunction|FindAPointtoGo))))))

(fn ConstructionScript
  (|CallParentFunction))