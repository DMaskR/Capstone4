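; Health pickup that bobs up and down and heals BP_MainCharacter when it overlaps the box.
; Two looping timers alternately interpolate the actor between its spawn location and a raised point, each handing off to the other near its target.
; Pickup is skipped when the character's IA flag is set; otherwise it adds health, then hides and ignores overlaps for a short delay before reappearing.
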(event OnComponentBeginOverlap(Box)
  (params (OverlappedComponent :type Primitive%20Component%20Object%20Reference) (OtherActor :type Actor%20Object%20Reference) (OtherComp :type Primitive%20Component%20Object%20Reference) (OtherBodyIndex :type Integer) (bFromSweep :type Boolean) (SweepResult :type Hit%20Result%20Structure%20%28by%20ref%29))
  (if (not (Variables|Default|GetDeactivate))
    (bind _asbp_main_character (Utilities|Casting|CastToBP_MainCharacter OtherActor))
    (if (not (Variables|/Game/Blueprints/BP_MainCharacter.BP_MainCharacter_C|GetIA _asbp_main_character))
      (Default|AddHealth _asbp_main_character (Variables|Default|GetHealthValue))
      (CallFunction|DeactiveMedkit))))

(event Custom|GoUp
  (Utilities|Time|SetTimerbyFunctionName 0 "StartUp" 0.01 true)
  (Utilities|Time|ClearTimerbyFunctionName 0 "StartDown"))

(event Custom|GoDown
  (Utilities|Time|SetTimerbyFunctionName 0 "StartDown" 0.01 true)
  (Utilities|Time|ClearTimerbyFunctionName 0 "StartUp"))

(event Custom|ActivateMedkit
  (Rendering|SetActorHiddenInGame false)
  (Variables|Default|SetDeactivate false))

(event Custom|DeactiveMedkit
  (Rendering|SetActorHiddenInGame true)
  (Variables|Default|SetDeactivate true)
  (Utilities|FlowControl|Delay 5.0)
  (CallFunction|ActivateMedkit))

(event EventBeginPlay
  (bind _returnvalue (Transformation|GetActorLocation))
  (Variables|Default|SetOriginLoc _returnvalue)
  (bind _output_get (Variables|Default|SetCurrentLoc _returnvalue))
  (Variables|Default|SetUpLoc (Math|Vector|MakeVector (.X (Math|Vector|BreakVector _output_get)) (.Y (Math|Vector|BreakVector _output_get)) (+ (.Z (Math|Vector|BreakVector _output_get)) 5e+01)))
  (CallFunction|GoUp))

(fn ConstructionScript)

(fn StartUp
  (bind _uploc (Variables|Default|GetUpLoc))
  (Variables|Default|SetCurrentLoc (Math|Interpolation|VInterpTo (Variables|Default|GetCurrentLoc) _uploc (Utilities|Time|GetWorldDeltaSeconds) (Variables|Default|GetInterp%20Speed)))
  (Transformation|SetActorLocation (Math|Interpolation|VInterpTo (Variables|Default|GetCurrentLoc) _uploc (Utilities|Time|GetWorldDeltaSeconds) (Variables|Default|GetInterp%20Speed)) false false)
  (if (Math|Vector|Equal(Vector) (Math|Interpolation|VInterpTo (Variables|Default|GetCurrentLoc) _uploc (Utilities|Time|GetWorldDeltaSeconds) (Variables|Default|GetInterp%20Speed)) _uploc 5.0)
    (Utilities|Time|ClearTimerbyFunctionName 0 "StartUp")
    (CallFunction|GoDown)))

(fn StartDown
  (bind _originloc (Variables|Default|GetOriginLoc))
  (Variables|Default|SetCurrentLoc (Math|Interpolation|VInterpTo (Variables|Default|GetCurrentLoc) _originloc (Utilities|Time|GetWorldDeltaSeconds) (Variables|Default|GetInterp%20Speed)))
  (Transformation|SetActorLocation (Math|Interpolation|VInterpTo (Variables|Default|GetCurrentLoc) _originloc (Utilities|Time|GetWorldDeltaSeconds) (Variables|Default|GetInterp%20Speed)) false false)
  (if (Math|Vector|Equal(Vector) (Math|Interpolation|VInterpTo (Variables|Default|GetCurrentLoc) _originloc (Utilities|Time|GetWorldDeltaSeconds) (Variables|Default|GetInterp%20Speed)) _originloc 5.0)
    (Utilities|Time|ClearTimerbyFunctionName 0 "StartDown")
    (CallFunction|GoUp)))